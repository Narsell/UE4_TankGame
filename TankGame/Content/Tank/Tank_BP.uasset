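; Tank pawn Blueprint that turns player input into aiming, driving and firing.
; On BeginPlay it hands the barrel and turret to TankAiming and both tracks to TankMovement.
; Movement axes pass forward and turn intent to TankMovement, while aim axes rotate separate yaw (ThetaRotation) and pitch (PhiRotation) components locally.
; The Fire action calls Fire, and the construction script only prints a debug message.
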(event EventBeginPlay
  (Class|TankAimingComponent|Initialize (Variables|Default|GetTankAiming) (Variables|Default|GetBarrel) (Variables|Default|GetTurret))
  (Class|TankMovementComponent|Initialize (Variables|Default|GetTankMovement) (Variables|Default|GetLeft_Track) (Variables|Default|GetRight_Track)))

(event Input|ActionEvents|InputActionFire
  (params (Key :type Key%20Structure :default "AnyKey"))
  ;[1 1 1] Aiming input binding
  (:Pressed
    (Class|Tank|Fire)))

(event Input|AxisEvents|InputAxisAimTheta
  (params (AxisValue :type Float%20%28single-precision%29))
  ;[1 1 1] Aiming input binding
  (Transformation|AddLocalRotation (Variables|Default|GetTheta%20Rotation) (Math|Rotator|MakeRotator 0.0 0.0 AxisValue) false false))

(event Input|AxisEvents|InputAxisTurnRight
  (params (AxisValue :type Float%20%28single-precision%29))
  ;[1 1 1] Movement Input Binding
  (Class|TankMovementComponent|IntendTurnRight (Variables|Default|GetTankMovement) AxisValue))

(event Input|AxisEvents|InputAxisAimPhi
  (params (AxisValue :type Float%20%28single-precision%29))
  ;[1 1 1] Aiming input binding
  (Transformation|AddLocalRotation (Variables|Default|GetPhi%20Rotation) (Math|Rotator|MakeRotator 0.0 AxisValue 0.0) false false))

(event Input|AxisEvents|InputAxisMoveForward
  (params (AxisValue :type Float%20%28single-precision%29))
  ;[1 1 1] Movement Input Binding
  (Class|TankMovementComponent|IntendMoveForward (Variables|Default|GetTankMovement) AxisValue))

(fn ConstructionScript
  (Development|PrintString "NORMIE: Tank_BP constructed"))